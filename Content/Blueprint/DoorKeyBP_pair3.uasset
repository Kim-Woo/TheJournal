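; DoorKeyBP_pair3 is a door key pickup, the third key by its flag, collected through an Interact function.
; When watched, Interact shows a DoorKeyWidget hint.
; Otherwise it swaps in a "got" widget, destroys the key, sets IsDoorKeyGet3 on the FirstPersonCharacter and plays a pickup sound at the player.
; The overlap-based hint and GameMode flag logic are left disconnected and unused.
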(event Collision|EventActorBeginOverlap
  (params (OtherActor :type Actor%20Object%20Reference))
  ;[1 1 1] Show Hint (not use anymore
)

(event Collision|EventActorEndOverlap
  (params (OtherActor :type Actor%20Object%20Reference)))

(fn ConstructionScript)

(fn Interact
  (params (isWatching :type Boolean))
  (bind _returnvalue (Game|GetPlayerCharacter 0))
  ;[1 1 1] Remove hint, show message, get the key
  (if isWatching
    ;[1 1 1] Show Hint
    (bind _returnvalue_2 (UserInterface|CreateWidget "/Game/Blueprint/DoorKeyWidget.DoorKeyWidget_C"))
    (Variables|Default|SetDoorKeyWidget _returnvalue_2)
    (Variables|/Game/Blueprint/DoorKeyWidget.DoorKeyWidget_C|SetisGot _returnvalue_2 (not true))
    (UserInterface|Viewport|AddtoViewport _returnvalue_2 0)
    (else
      (Widget|RemovefromParent (Variables|Default|GetDoorKeyWidget))
      (bind _returnvalue_3 (UserInterface|CreateWidget "/Game/Blueprint/DoorKeyWidget.DoorKeyWidget_C"))
      (Variables|Default|SetDoorKeyWidget _returnvalue_3)
      (Variables|/Game/Blueprint/DoorKeyWidget.DoorKeyWidget_C|SetisGot _returnvalue_3 true)
      (UserInterface|Viewport|AddtoViewport _returnvalue_3 0)
      (Actor|DestroyActor)
      (bind _asfirst_person_character (Utilities|Casting|CastToFirstPersonCharacter _returnvalue))
      (Variables|/Game/FirstPersonBP/Blueprints/FirstPersonCharacter.FirstPersonCharacter_C|SetisDoorKeyGet_3 _asfirst_person_character true)
      (Audio|PlaySoundatLocation "/Game/Sound/KeyGetSound.KeyGetSound" (Transformation|GetActorLocation _returnvalue) "0, 0, 0" 1.0 1.0 0.0 0 0 0)))
  (return true))