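; DoorKeyBP is a door key pickup that shows a hint and is collected through interaction.
; Overlapping it creates a DoorKeyWidget and fades the hint in, then back out after a short delay.
; Interact swaps that widget for one flagged as got, destroys the actor and sets IsDoorKey1Get on FirstPersonCharacter.
; An older path that stored the flag on TheGameMode remains unconnected.
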(event Collision|EventActorBeginOverlap
  (params (OtherActor :type Actor%20Object%20Reference))
  ;[1 1 1] Show Hint
  (bind _returnvalue (UserInterface|CreateWidget "/Game/Blueprint/DoorKeyWidget.DoorKeyWidget_C"))
  (Variables|Default|SetDoorKeyWidget _returnvalue)
  (UserInterface|Viewport|AddtoViewport _returnvalue 0)
  (UserInterface|Animation|PlayAnimation _returnvalue (Variables|/Game/Blueprint/DoorKeyWidget.DoorKeyWidget_C|GetHintFade _returnvalue) 0.0 1 "Forward" 1.0 false)
  (Utilities|FlowControl|Delay 2.0)
  (UserInterface|Animation|PlayAnimation _returnvalue (Variables|/Game/Blueprint/DoorKeyWidget.DoorKeyWidget_C|GetHintFade _returnvalue) 0.0 1 "Reverse" 1.0 false)
  (Utilities|FlowControl|Delay 0.3))

(event Collision|EventActorEndOverlap
  (params (OtherActor :type Actor%20Object%20Reference)))

(fn ConstructionScript)

(fn Interact
  ;[1 1 1] Remove hint, show message, get the key
  (Widget|RemovefromParent (Variables|Default|GetDoorKeyWidget))
  (bind _returnvalue (UserInterface|CreateWidget "/Game/Blueprint/DoorKeyWidget.DoorKeyWidget_C"))
  (Variables|/Game/Blueprint/DoorKeyWidget.DoorKeyWidget_C|SetisGot _returnvalue true)
  (UserInterface|Viewport|AddtoViewport _returnvalue 0)
  (Actor|DestroyActor)
  (bind _asfirst_person_character (Utilities|Casting|CastToFirstPersonCharacter (Game|GetPlayerCharacter 0)))
  (Variables|/Game/FirstPersonBP/Blueprints/FirstPersonCharacter.FirstPersonCharacter_C|SetisDoorKey1Get _asfirst_person_character true)
  (return true))