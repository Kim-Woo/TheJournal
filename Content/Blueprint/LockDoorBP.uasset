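; A locked door Blueprint that swings open when the player interacts with it while holding the first key.
; Interact casts the player character to FirstPersonCharacter, checks its IsDoorKey1Get flag, then plays the OpenDoor timeline and returns true.
; The timeline's update lerps the Door's relative yaw between the closed and open angles, with no logic to close it again.
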(fn ConstructionScript)

(fn Interact
  (bind _asfirst_person_character (Utilities|Casting|CastToFirstPersonCharacter (Game|GetPlayerCharacter 0)))
  (if (Variables|/Game/FirstPersonBP/Blueprints/FirstPersonCharacter.FirstPersonCharacter_C|GetisDoorKey1Get _asfirst_person_character)
    (Audio|Components|Audio|Play (Variables|Default|GetOpen%20Door))
    (return true)))