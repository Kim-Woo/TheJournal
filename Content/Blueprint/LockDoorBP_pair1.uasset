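; Locked door Blueprint that opens only when the first-person character holds its key.
; Interact, when IsWatching is false, checks the character's IsDoorKeyGet1 flag, then either plays the OpenDoor timeline and returns true or plays a locked sound at the player.
; The timeline's DoorTrack lerps the door's relative yaw between closed and open angles.
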(fn ConstructionScript)

(fn Interact
  (params (isWatching :type Boolean))
  (bind _returnvalue (Game|GetPlayerCharacter 0))
  (if (not isWatching)
    (bind _asfirst_person_character (Utilities|Casting|CastToFirstPersonCharacter _returnvalue))
    (if (Variables|/Game/FirstPersonBP/Blueprints/FirstPersonCharacter.FirstPersonCharacter_C|GetisDoorKeyGet_1 _asfirst_person_character)
      (Audio|Components|Audio|Play (Variables|Default|GetOpen%20Door))
      (return true)
      (else
        (Audio|PlaySoundatLocation "/Game/Sound/DoorLocked.DoorLocked" (Transformation|GetActorLocation _returnvalue) "0, 0, 0" 1.0 1.0 0.0 0 0 0)))))